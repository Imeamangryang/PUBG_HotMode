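; MetaHuman-style character Blueprint that assembles modular skeletal meshes and optionally drives the body mesh from Live Link.
; The construction script makes body child meshes, except the face, follow the body's pose unless they have their own animation Blueprint.
; With Live Link on, the body uses either ABP_MH_LiveLink for ARKit or a plain LiveLinkInstance.
; Face or body anim initialization assigns the subject and toggles in-editor animation updates to match.
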(event OnAnimInitialized(Body_0)
  ;[1 1 1] Live Link Setup
  (CallFunction|LiveLinkSetup (Variables|Default|GetBody_0) (Variables|LiveLink|GetLiveLinkSubject_0) 0 (Variables|LiveLink|GetUseLiveLink_0))
  (CallFunction|SetUpdateAnimationinEditor (or false (Variables|LiveLink|GetUseLiveLink_0))))

(event OnAnimInitialized(Face_0)
  ;[1 1 1] Live Link Setup
  (CallFunction|LiveLinkSetup (Variables|Default|GetBody_0) (Variables|LiveLink|GetLiveLinkSubject_0) 0 (Variables|LiveLink|GetUseLiveLink_0))
  (CallFunction|SetUpdateAnimationinEditor (or false (Variables|LiveLink|GetUseLiveLink_0))))

(event EventBeginPlay)

(event Collision|EventActorBeginOverlap
  (params (OtherActor :type Actor%20Object%20Reference)))

(event EventTick
  (params (DeltaSeconds :type Float%20%28single-precision%29)))

(fn ConstructionScript
  (bind _body_0 (Variables|Default|GetBody_0))
  (for _array_element (Components|GetChildrenComponents (Variables|Default|GetBody_0) false)
    (bind _as스켈레탈_메시_컴포넌트 (Utilities|Casting|CastToSkeletalMeshComponent _array_element))
    (if (!= _as스켈레탈_메시_컴포넌트 (Variables|Default|GetFace_0))
      (CallFunction|EnableMasterPose _as스켈레탈_메시_컴포넌트)))
  (if (Variables|LiveLink|GetUseLiveLink_0)
    (if (Variables|LiveLink|GetUseARKit_0)
      (Components|SkeletalMesh|SetAnimInstanceClass _body_0 "/Game/MetaHumans/Common/Animation/ABP_MH_LiveLink.ABP_MH_LiveLink_C")
      (else
        (Components|SkeletalMesh|SetAnimInstanceClass _body_0 "/Script/LiveLinkAnimationCore.LiveLinkInstance")))))

(fn EnableMasterPose
  (params (SkeletalMeshComponent :type Skeletal%20Mesh%20Component%20Object%20Reference))
  (bind _returnvalue (Components|SkeletalMesh|GetSkeletalMeshAsset SkeletalMeshComponent))
  (if (Utilities|IsValid _returnvalue)
    (if (not (or (Utilities|IsValidClass (Variables|/Script/Engine.SkeletalMesh|GetPostProcessAnimBlueprint _returnvalue)) (Utilities|IsValidClass (Variables|/Script/Engine.SkeletalMeshComponent|GetAnimClass SkeletalMeshComponent))))
      (Components|SkinnedMesh|SetLeaderPoseComponent SkeletalMeshComponent (Variables|Default|GetBody_0) false false))))

(fn LiveLinkSetup
  (params (SkeletalMesh :type Skeletal%20Mesh%20Component%20Object%20Reference) (SubjectName :type Live%20Link%20Subject%20Name%20Structure) (RetargetAsset :type Live%20Link%20Retarget%20Asset%20Class%20Reference) (UseLiveLink :type Boolean))
  (bind _returnvalue (Components|SkeletalMesh|GetAnimInstance SkeletalMesh))
  (if UseLiveLink
    (if (Variables|LiveLink|GetUseARKit_0)
      (bind _asabp_mh_live_link (Utilities|Casting|CastToABP_MH_LiveLink _returnvalue))
      (Variables|/Game/MetaHumans/Common/Animation/ABP_MH_LiveLink.ABP_MH_LiveLink_C|SetLLink_Face_Subj _asabp_mh_live_link SubjectName)
      (else
        (bind _as라이브_링크_인스턴스 (Utilities|Casting|CastToLiveLinkInstance _returnvalue))
        (Class|LiveLinkInstance|SetSubject _as라이브_링크_인스턴스 SubjectName)
        (Class|LiveLinkInstance|SetRetargetAsset _as라이브_링크_인스턴스 RetargetAsset)))))

(fn SetUpdateAnimationinEditor
  (params (IsEnabled :type Boolean))
  (for _array_element (Components|GetChildrenComponents (Variables|Default|GetRoot_0) true)
    (bind _as스켈레탈_메시_컴포넌트 (Utilities|Casting|CastToSkeletalMeshComponent _array_element))
    (Components|SkeletalMesh|SetUpdateAnimationinEditor _as스켈레탈_메시_컴포넌트 IsEnabled)))